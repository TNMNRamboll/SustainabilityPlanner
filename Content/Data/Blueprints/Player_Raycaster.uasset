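; Player raycaster Blueprint that lets the user click to select Vitruvio plots in the world.
; On BeginPlay it enables input and selects the default actor's Vitruvio component.
; When raycasting is enabled, left click traces from the mouse, stores any hit VitruvioActor component with valid input data and signals plot selection.
; GetAttributeNames rebuilds slider bound maps from the default actor's attributes, skipping ignored ones and assigning fixed ranges.
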(event EventBeginPlay
  (Input|EnableInput (Game|GetPlayerController 0))
  (Variables|Default|SetSelectedVitComponent (Variables|/Script/Vitruvio.VitruvioActor|GetVitruvioComponent (Variables|Default|GetDefaultVitActor))))

(event Input|MouseEvents|LeftMouseButton
  (params (Key :type Key%20Structure :default "None"))
  (bind _returnvalue (Game|GetPlayerController 0))
  (bind (_worldlocation _worlddirection) (Game|Player|ConvertMouseLocationToWorldSpace _returnvalue))
  (:Pressed
    (if (Variables|Default|GetRaycastEnabled)
      (bind _outhit (Collision|LineTraceByChannel _worldlocation (+ _worldlocation (* _worlddirection 1e+05)) "TraceTypeQuery1" false (Variables|Default|GetRaycastIgnoreActors) "None"))
      (bind _asvitruvio_actor (Utilities|Casting|CastToVitruvioActor (.HitActor (Collision|BreakHitResult _outhit))))
      (if (Class|VitruvioComponent|HasValidInputData (Variables|/Script/Vitruvio.VitruvioActor|GetVitruvioComponent _asvitruvio_actor))
        (Variables|Default|SetSelectedVitComponent (Variables|/Script/Vitruvio.VitruvioActor|GetVitruvioComponent _asvitruvio_actor))
        (Default|CallOnPlotSelected)))))

(fn ConstructionScript)

(fn GetAttributeNames
  (Utilities|Map|Clear (Variables|Default|GetSlider%20Attributes%20Min%20Bounds))
  (Utilities|Map|Clear (Variables|Default|GetSlider%20Attributes%20Max%20Bounds))
  (bind _keys (Utilities|Map|Keys (Class|VitruvioComponent|GetAttributes (Variables|/Script/Vitruvio.VitruvioActor|GetVitruvioComponent (Variables|Default|GetDefaultVitActor)))))
  (for _array_element _keys
    (LocalVariables|SetAttribute _array_element)
    (if (== (Utilities|Array|FindItem (Variables|Default|GetIgnored%20Slider%20Attributes) (LocalVariables|GetAttribute)) -1)
      (Utilities|Map|Add (Variables|Default|GetSlider%20Attributes%20Min%20Bounds) (LocalVariables|GetAttribute) 0)
      (Utilities|Map|Add (Variables|Default|GetSlider%20Attributes%20Max%20Bounds) (LocalVariables|GetAttribute) 10))))